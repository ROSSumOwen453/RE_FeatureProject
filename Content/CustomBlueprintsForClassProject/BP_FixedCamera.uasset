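; BP_FixedCamera is a fixed-camera trigger that blends the player's view to itself when the player character enters its Box volume.
; Box overlap calls OnFixedCameraOverlap, which sets this actor as the player controller's view target using configurable blend time and function.
; A check shortly after BeginPlay triggers the same switch if the player starts inside the box.
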(event `self.Box.OnComponentBeginOverlap`
  (params (OverlappedComponent :type "PrimitiveComponent Object Reference") (OtherActor :type "Actor Object Reference") (OtherComp :type "PrimitiveComponent Object Reference") (OtherBodyIndex :type Integer) (bFromSweep :type Boolean) (SweepResult :type "HitResult Structure (by ref)"))
  ;[0 1 0.09208] when player collides with camera box collsion
  (if (== OtherActor (`GameplayStatics.GetPlayerCharacter` 0))
    (`self.OnFixedCameraOverlap` :!label _label)))

(event `self.ReceiveBeginPlay`
  ;[0.1417 1 0] when player starts in side the box collider at spawn
  (`KismetSystemLibrary.Delay` 0.5)
  (if (`PrimitiveComponent.IsOverlappingActor` (`self.Box`) (`GameplayStatics.GetPlayerCharacter` 0))
    (goto _label)))

(fn `OnFixedCameraOverlap`
  (`PlayerController.SetViewTargetWithBlend` (`GameplayStatics.GetPlayerController` 0) self (`self.Blend Time`) (`self.Blend Func`) 0.0 false))

(fn `UserConstructionScript`)